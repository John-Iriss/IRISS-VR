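; Ultrasound emitter Blueprint that plays a looping sound at its root location, with volume driven by distance and angle modifiers.
; A timeline starts on BeginPlay; each update spawns the audio if absent, otherwise sets its volume to (1 + DistanceMod) × (1 − AngleMod).
; When the timeline finishes, it destroys the audio component and restarts itself.
; The timeline's amplitude is stored in DB but does not affect volume, and both modifiers are only read here.
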(event `self.ReceiveBeginPlay`
  (bind _currentaudio (`self.CurrentAudio`))
  (bind _soundmultiplier (`self.SoundMultiplier`))
  ;[1 1 1] Play sound with Amp timeline...
  (bind (_direction _amp) (`Timeline|SonusSound-01` :!label _label)
    (:`Update`
      (set `self.dB` _amp)
      (set `self.SoundMultiplier` (* (+ 1.0 (`self.DistanceMod`)) (- 1.0 (`self.AngleMod`))))
      ;[1 1 1] If there is an existing sound...
      (if (`KismetSystemLibrary.IsValid` _currentaudio)
        ;[1 1 1] Set multiplier
        (`AudioComponent.SetVolumeMultiplier` _currentaudio _soundmultiplier)
        (else
          ;[1 1 1] Spawn new sound...
          (bind _returnvalue (`GameplayStatics.SpawnSoundAtLocation` (`self.UltrasoundFile`) (`SceneComponent.K2_GetComponentLocation` (`self.DefaultSceneRoot`)) (struct) _soundmultiplier 1.0 0.0 null null false))
          (set `self.CurrentAudio` _returnvalue))))
    (:`Finished`
      (`ActorComponent.K2_DestroyComponent` _currentaudio)
      (goto _label :!via `PlayFromStart`))))

(fn `UserConstructionScript`)
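; BP-SonusXT is a motion-controller pickup that acts as a directional ultrasound listening device.
; Pickup disables physics, attaches it to the given component and starts Listen; Drop detaches it and restores physics without stopping Listen.
; Listen loops on a short Delay, writing DistanceMod and AngleMod to each Ultrasound-tagged UltrasoundEmission actor.
; CosineCalc derives these from clamped, scaled distance and a law-of-cosines angle between the device's forward vector and the source.
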(event `/Game/Blueprints/PickupActorInterface.Pickup`
  (params (AttachTo :type "SceneComponent Object Reference"))
  (`PrimitiveComponent.SetSimulatePhysics` (`self.StaticMeshComponent`) false)
  (`SceneComponent.K2_AttachToComponent` (`self.K2_GetRootComponent`) AttachTo "None" "SnapToTarget" "SnapToTarget" "KeepWorld" false)
  ;[1 1 1] Listen if device is attached
  (`self.Listen`))

(event `/Game/Blueprints/PickupActorInterface.Drop`
  (`PrimitiveComponent.SetSimulatePhysics` (`self.StaticMeshComponent`) true)
  (`self.K2_DetachFromActor` "KeepWorld" "KeepWorld" "KeepWorld"))

(event `Listen`
  ;[1 1 1] Get all ultrasound actors with Delay and get distance and angle from source.
  (bind _outactors (`GameplayStatics.GetAllActorsWithTag` "Ultrasound" :!label _label))
  (for _array_element _outactors
    ;[1 1 1] Run Cosine Calculations
    (bind (_distancemod _anglemod) (`self.CosineCalc` _array_element))
    ;[1 1 1] Cast and set parameters...
    (bind _asultrasound_emission (cast `/Game/Blueprints/Sonus/UltrasoundEmission` _array_element))
    (set `/Game/Blueprints/Sonus/UltrasoundEmission.DistanceMod` _distancemod _asultrasound_emission)
    (set `/Game/Blueprints/Sonus/UltrasoundEmission.AngleMod` _anglemod _asultrasound_emission))
  (`KismetSystemLibrary.Delay` 0.2)
  (goto _label))

(fn `CosineCalc`
  (params (SoundActor :type "Actor Object Reference"))
  (returns (DistanceMod :type "Float (double-precision)") (AngleMod :type "Float (double-precision)"))
  (bind _b (`self.B`))
  (bind _returnvalue (`self.GetDistanceTo` SoundActor self))
  (bind _returnvalue_2 (`KismetMathLibrary.Square` _b))
  ;[1 1 1] Get distance to sound divided...
  (bind _result (`/Engine/EditorBlueprintResources/StandardMacros.NegateFloat` (/ _returnvalue 1000.0))
    (:`  `
      (set `self.B` _returnvalue)
      (return (`KismetMathLibrary.FClamp` _result -1.0 0.0) (`KismetMathLibrary.Lerp` 0.0 1.0 (/ (`KismetMathLibrary.DegAcos` (/ (- (+ _returnvalue_2 _returnvalue_2) (`KismetMathLibrary.Square` (`KismetMathLibrary.VSize` (- (+ (`self.K2_GetActorLocation` self) (* (`KismetMathLibrary.GetForwardVector` (`self.K2_GetActorRotation` self)) _returnvalue)) (`self.K2_GetActorLocation` SoundActor))))) (* 2.0 (* _b (`self.B`))))) 180.0))))))

(fn `UserConstructionScript`)
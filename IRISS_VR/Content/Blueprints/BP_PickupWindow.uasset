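; BP_PickupWindow is a window that motion controllers pick up, drop and install into a BP_SwitchPanel.
; On hit or overlap with a panel in Cutout state, it snaps on, turns off panel physics, sets its own collision to overlap and marks both states finished.
; Pickup attaches it to the hand until installed, then instead toggles it open or closed through a FlipFlop between a hard-coded transform and the BeginPlay transform.
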(event `self.ReceiveHit`
  (params (MyComp :type "PrimitiveComponent Object Reference") (Other :type "Actor Object Reference") (OtherComp :type "PrimitiveComponent Object Reference") (bSelfMoved :type Boolean) (HitLocation :type "Vector Structure") (HitNormal :type "Vector Structure") (NormalImpulse :type "Vector Structure") (Hit :type "HitResult Structure (by ref)"))
  ;[1 1 1] When this object hits or overlaps a SwitchPanel that has PanelState (String Var) = Cutout, attach to actor with adjustment (positioning relative) and disable physics and change collision channels. When finished, change PanelState and WindowState
  (bind _asbp_switch_panel (cast `/Game/Blueprints/BP_SwitchPanel` Other :!label _label))
  (if (`KismetStringLibrary.EqualEqual_StrStr` (`/Game/Blueprints/BP_SwitchPanel.PanelState` _asbp_switch_panel) "Cutout")
    (`self.K2_AttachToActor` _asbp_switch_panel "None" "SnapToTarget" "SnapToTarget" "KeepWorld")
    (`SceneComponent.K2_SetRelativeLocationAndRotation` (`self.StaticMeshComponent`) (0.0 3.0 -38.0) (struct :`Pitch` 180.0 :`Yaw` 180.0) false true)
    (`PrimitiveComponent.SetSimulatePhysics` (`StaticMeshActor.StaticMeshComponent` _asbp_switch_panel) false)
    (`PrimitiveComponent.SetCollisionResponseToAllChannels` (`self.StaticMeshComponent`) "ECR_Overlap")
    (set `/Game/Blueprints/BP_SwitchPanel.PanelState` "Complete" _asbp_switch_panel)
    (set `self.WindowState` "Installed")))

(event `self.ReceiveActorBeginOverlap`
  (params (OtherActor :type "Actor Object Reference"))
  ;[1 1 1] When this object hits or overlaps a SwitchPanel that has PanelState (String Var) = Cutout, attach to actor with adjustment (positioning relative) and disable physics and change collision channels. When finished, change PanelState and WindowState
  (goto _label))

(event `/Game/Blueprints/PickupActorInterface.Pickup`
  (params (AttachTo :type "SceneComponent Object Reference"))
  ;[1 1 1] Altered Motion Controller Pickup Script : When a motion controller (Vive/Oculus) tries a pick-up action, check WindowState if it is NOTinstalled. If yes, it can be picked up, if not, it can be opened instead.
  (if (`KismetStringLibrary.NotEqual_StrStr` (`self.WindowState`) "Installed")
    (`PrimitiveComponent.SetSimulatePhysics` (`self.StaticMeshComponent`) false)
    (`SceneComponent.K2_AttachToComponent` (`self.K2_GetRootComponent`) AttachTo "None" "KeepWorld" "KeepWorld" "KeepWorld" false)
    (else
      (`self.OpenClose`))))

(event `/Game/Blueprints/PickupActorInterface.Drop`
  ;[1 1 1] When a motion controller lets go of this object, it detaches from the 'hand' and physics is enabled.
  (`PrimitiveComponent.SetSimulatePhysics` (`self.StaticMeshComponent`) true)
  (`self.K2_DetachFromActor` "KeepWorld" "KeepWorld" "KeepWorld"))

(event `OpenClose`
  (bind _staticmesh (`self.StaticMesh`))
  ;[1 1 1] When installed, 'picking up' the window will swap it from being opened or closed. This was a hack together transform that moved the door opened or closed. A prettier solution with animations or physical manipulation may be a good improvement.
  (`/Engine/EditorBlueprintResources/StandardMacros.FlipFlop`
    (:`A`
      (`SceneComponent.K2_SetRelativeTransform` _staticmesh (`KismetMathLibrary.MakeTransform` (0.0 -16.299999 14.45) (struct :`Roll` 90.0)) false false))
    (:`B`
      (`SceneComponent.K2_SetRelativeTransform` _staticmesh (stale `self.ReceiveBeginPlay` _output_get) false false))))

(event `self.ReceiveBeginPlay`
  ;[1 1 1] When installed, 'picking up' the window will swap it from being opened or closed. This was a hack together transform that moved the door opened or closed. A prettier solution with animations or physical manipulation may be a good improvement.
  ;;[1 1 1] Sets the starting position.
  (bind _output_get (set `self.StartTransform` (`SceneComponent.GetRelativeTransform` (`self.StaticMesh`)))))

(fn `UserConstructionScript`)
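; SummonItem is an actor meant to return its assigned SceneActor to a saved transform when a BP_MotionController overlaps it.
; Setup logic caches that actor's transform and shows its name on a TextRender label.
; The summon logic teleports the actor back without sweep, skipping any BP_PickupWindow whose state is Installed.
; Both logic chains are disconnected from BeginPlay and ActorBeginOverlap, so neither runs as the graph stands.
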(event `self.ReceiveBeginPlay`
  ;[1 1 1] Find the scene actor assgined to this summon item BP. Get its current transform and set as Actor Transform, then get its name for the label.
)

(event `self.ReceiveActorBeginOverlap`
  (params (OtherActor :type "Actor Object Reference"))
  ;[1 1 1] When a motion controller (hand) overlaps this detector, and its scene actor is valid, return true.
)

(fn `UserConstructionScript`)
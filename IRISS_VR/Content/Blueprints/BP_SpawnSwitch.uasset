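; BP_SpawnSwitch is a one-shot switch that spawns its assigned gear as part of a gear selection.
; Pickup, while Useable, turns the cube green and passes GearToSpawn to the first BP_GearSpawn found.
; It then calls Deactivated on every switch, itself included, which blacks out the cube, disables use and destroys BP_GearSelectionMenu actors.
; The construction script caches spawn points, which Pickup does not use, and applies TypeTag.
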(event `/Game/Blueprints/PickupActorInterface.Pickup`
  (params (AttachTo :type "SceneComponent Object Reference"))
  (if (`self.Useable`)
    (`PrimitiveComponent.SetMaterial` (`self.Cube`) 0 "/Game/Materials/Green.Green")
    (bind _outactors (`GameplayStatics.GetAllActorsOfClass` "/Game/Blueprints/BP_GearSpawn.BP_GearSpawn_C"))
    (`/Game/Blueprints/BP_GearSpawn.SpawnGear` (`|GetArrayItem` _outactors) (`self.GearToSpawn`))
    (bind _outactors_2 (`GameplayStatics.GetAllActorsOfClass` "BP_SpawnSwitch_C"))
    (for _array_element _outactors_2
      (bind _asbp_spawn_switch (cast `/Game/Blueprints/BP_SpawnSwitch` _array_element))
      (`self.Deactivated` _asbp_spawn_switch))))

(event `Deactivated`
  (`PrimitiveComponent.SetMaterial` (`self.Cube`) 0 "/Game/Import/AG_Black.AG_Black")
  (set `self.Useable` false)
  (bind _outactors (`GameplayStatics.GetAllActorsOfClass` "/Game/Blueprints/BP_GearSelectionMenu.BP_GearSelectionMenu_C"))
  (`self.K2_DestroyActor` _outactors))

(fn `UserConstructionScript`
  (bind _outactors (`GameplayStatics.GetAllActorsOfClass` "/Game/Blueprints/BP_GearSpawn.BP_GearSpawn_C"))
  (set `self.SpawnPoint` _outactors)
  (set `self.Tags` (`|MakeArray` (`self.Type Tag`))))
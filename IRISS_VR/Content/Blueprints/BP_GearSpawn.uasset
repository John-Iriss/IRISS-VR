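; BP_GearSpawn spawns a gear actor and slides it from a start point to an end point.
; BeginPlay caches the world locations of the SpawnPoint and EndPoint components.
; The SpawnGear event spawns the given gear class at the start location.
; A timeline then lerps the new actor's location toward the end point each update, without sweeping.
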(event `self.ReceiveBeginPlay`
  (set `self.SpawnLocation` (`SceneComponent.K2_GetComponentLocation` (`self.SpawnPoint`)))
  (set `self.EndLocation` (`SceneComponent.K2_GetComponentLocation` (`self.EndPoint`))))

(event `SpawnGear`
  (params (Gear :type "Actor Class Reference"))
  (bind _returnvalue (`|SpawnActorFromClass` Gear (`KismetMathLibrary.Conv_VectorToTransform` (`self.SpawnLocation`)) "Undefined" "OverrideRootScale" null null))
  (bind (_direction _movespeed) (`Timeline|Timeline_0` :!via `PlayFromStart`)
    (:`Update`
      (`self.K2_SetActorLocation` _returnvalue (`KismetMathLibrary.VLerp` (`self.SpawnLocation`) (`self.EndLocation`) _movespeed) false false))))

(fn `UserConstructionScript`)
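; BP_SwitchPanel is a VR-grabbable switchgear panel that gets unbolted, cut out for a window template and bolted back on.
; Child bolts gathered at construction gate pickup, which attaches the panel to the motion controller.
; Cutout swaps the mesh and spawns the template, after which overlapping switchgear snaps the panel on.
; Milestones notify BP_GameMode_IRISS, mostly once, and full rebolting releases the lockout tag.
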(event `TemplateAttached`
  (params (`Cutout Panel` :type "StaticMesh Object Reference") (`Cutout Template` :type "Actor Class Reference"))
  ;[1 1 1] Attach and cut out template
  (set `self.Cut Out Panel` `Cutout Panel`)
  (set `self.Cutout Template` `Cutout Template`)
  (`/Engine/EditorBlueprintResources/StandardMacros.DoOnce` false
    (:`Completed`
      (`/Game/Blueprints/BP_GameMode_IRISS.TemplateOn` (cast `/Game/Blueprints/BP_GameMode_IRISS` (`GameplayStatics.GetGameMode`) :!pure true)))))

(event `TemplateCutout`
  ;[1 1 1] Attach and cut out template
  (`StaticMeshComponent.SetStaticMesh` (`self.StaticMeshComponent`) (`self.Cut Out Panel`))
  (set `self.Tags` (`|MakeArray` (`self.Cutout Tag`)))
  (bind _returnvalue (`|SpawnActorFromClass` (`self.Cutout Template`) (`SceneComponent.GetSocketTransform` (`self.StaticMeshComponent`) "Window" "RTS_World") "Undefined" "OverrideRootScale" null null))
  (`self.K2_AttachToActor` _returnvalue self "Template" "SnapToTarget" "SnapToTarget" "KeepRelative" true)
  (set `self.CutOut` true)
  (`/Game/Blueprints/BP_GameMode_IRISS.HoleCut` (cast `/Game/Blueprints/BP_GameMode_IRISS` (`GameplayStatics.GetGameMode`) :!pure true)))

(event `/Game/Blueprints/PickupActorInterface.Pickup`
  (params (AttachTo :type "SceneComponent Object Reference"))
  (bind _returnvalue (`self.K2_GetRootComponent`))
  (bind _staticmeshcomponent (`self.StaticMeshComponent`))
  ;[1 1 1] If the panel is unbolted and a pickup is attempted, attach to motion controller, if released, drop motion controller. Grabbing is set/unset to prevent auto snapping to the SnapPoint BP
  (if (`self.UnboltedPanel`)
    (if (not (`self.Attached`))
      (`PrimitiveComponent.SetSimulatePhysics` _staticmeshcomponent false)
      (`SceneComponent.K2_AttachToComponent` _returnvalue AttachTo "None" "KeepWorld" "KeepWorld" "KeepWorld" false)
      (set `self.Grabbing` true)
      (else
        (`self.K2_DetachFromActor` "KeepWorld" "KeepWorld" "KeepWorld")
        (`PrimitiveComponent.SetSimulatePhysics` _staticmeshcomponent false)
        (`SceneComponent.K2_AttachToComponent` _returnvalue AttachTo "None" "KeepWorld" "KeepWorld" "KeepWorld" false)
        (set `self.Grabbing` true)))))

(event `self.Box.OnComponentBeginOverlap`
  (params (OverlappedComponent :type "PrimitiveComponent Object Reference") (OtherActor :type "Actor Object Reference") (OtherComp :type "PrimitiveComponent Object Reference") (OtherBodyIndex :type Integer) (bFromSweep :type Boolean) (SweepResult :type "HitResult Structure (by ref)"))
  ;[1 1 1] Attach Panel to Switch Gear
  (if (`self.CutOut`)
    (if (`self.ActorHasTag` OtherActor "SwitchGear")
      (`self.K2_AttachToActor` OtherActor "None" "SnapToTarget" "SnapToTarget" "KeepRelative" false)
      (set `self.Attached` true)
      (`/Engine/EditorBlueprintResources/StandardMacros.DoOnce` false
        (:`Completed`
          (`/Game/Blueprints/BP_GameMode_IRISS.PanelOn` (cast `/Game/Blueprints/BP_GameMode_IRISS` (`GameplayStatics.GetGameMode`) :!pure true)))))))

(event `/Game/Blueprints/PickupActorInterface.Drop`
  ;[1 1 1] If the panel is unbolted and a pickup is attempted, attach to motion controller, if released, drop motion controller. Grabbing is set/unset to prevent auto snapping to the SnapPoint BP
  (`PrimitiveComponent.SetSimulatePhysics` (`self.StaticMeshComponent`) true)
  (`self.K2_DetachFromActor` "KeepWorld" "KeepWorld" "KeepWorld")
  (set `self.Grabbing` false))

(event `Remove Bolt`
  (params (Bolt :type "Actor Object Reference"))
  ;[1 1 1] Add and remove bolts
  (`KismetArrayLibrary.Array_RemoveItem` (`self.Bolts`) Bolt)
  (if (<= (`KismetArrayLibrary.Array_Length` (`self.Bolts`)) 0)
    (set `self.UnboltedPanel` true)
    (`/Engine/EditorBlueprintResources/StandardMacros.DoOnce` false
      (:`Completed`
        (`/Game/Blueprints/BP_GameMode_IRISS.Bolts Removed` (cast `/Game/Blueprints/BP_GameMode_IRISS` (`GameplayStatics.GetGameMode`) :!pure true))))))

(event `Add Bolt`
  (params (Bolt :type "Actor Object Reference"))
  ;[1 1 1] Add and remove bolts
  (`KismetArrayLibrary.Array_Add` (`self.Bolts`) Bolt)
  (if (>= (`KismetArrayLibrary.Array_Length` (`self.Bolts`)) 1)
    (set `self.UnboltedPanel` false)
    (`/Engine/EditorBlueprintResources/StandardMacros.DoOnce` false :!label _label
      (:`Completed`
        (if (>= (`KismetArrayLibrary.Array_Length` (`self.Bolts`)) 4)
          (`/Game/Blueprints/BP_GameMode_IRISS.PanelBolted` (cast `/Game/Blueprints/BP_GameMode_IRISS` (`GameplayStatics.GetGameMode`) :!pure true))
          (bind _outactors (`GameplayStatics.GetAllActorsOfClass` "/Game/Blueprints/BP_LockoutTag.BP_LockoutTag_C"))
          (`/Game/Blueprints/BP_LockoutTag.SafeToRemove` (`|GetArrayItem` _outactors))
          (else
            (goto _label :!via `Reset`)))))))

(fn `UserConstructionScript`
  ;[1 1 1] Set Tag for Self
  (set `self.Tags` (`|MakeArray` (`self.TagName`)))
  ;[1 0.7565 0] JUST GET CHILD BOLTS
  (for _array_element (`self.GetAllChildActors` true)
    (if (`self.ActorHasTag` _array_element "Bolt")
      (`KismetArrayLibrary.Array_Add` (`self.Bolts`) _array_element))))
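; BP_Drill is a motion-controller pickup drill that removes and re-adds bolts or adds holes, depending on whether its bit is shown.
; Pickup attaches it and records the hand, so only that hand's trigger works; Drop destroys it.
; The swap action toggles the bit, selecting which collider's overlaps receive calls: hidden BP_Holes or "Bolt"-tagged actors.
; Outline events add or remove a duplicate mesh with outline materials.
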(event `self.ReceiveBeginPlay`)

(event `Create Outline`
  (if (not (`self.HasOutline`))
    (bind _returnvalue (`AddComponent|NODE_AddStaticMeshComponent-0` :`bManualAttachment` true :`RelativeTransform` (`SceneComponent.K2_GetComponentToWorld` (`self.Body`))))
    (bind _output_get (set `self.MeshComponent` _returnvalue))
    (`StaticMeshComponent.SetStaticMesh` _output_get (`self.Mesh`))
    (`SceneComponent.K2_AttachToComponent` (`self.MeshComponent`) (`self.Body`) "None" "KeepWorld" "KeepWorld" "KeepWorld" true)
    (`PrimitiveComponent.CreateDynamicMaterialInstance` _output_get 10 "/Game/Materials/Outlines/M_Outline.M_Outline" "None")
    (`PrimitiveComponent.CreateDynamicMaterialInstance` _output_get 8 "/Game/Materials/Outlines/M_Outline.M_Outline" "None")
    (`PrimitiveComponent.CreateDynamicMaterialInstance` _output_get 7 "/Game/Materials/Outlines/M_Outline.M_Outline" "None")
    (set `self.HasOutline` true)))

(event `Delete Outline`
  (bind _meshcomponent (`self.MeshComponent`))
  (`/Engine/EditorBlueprintResources/StandardMacros.IsValid` _meshcomponent
    (:`Is Valid`
      (`ActorComponent.K2_DestroyComponent` _meshcomponent)
      (set `self.HasOutline` false))))

(event `/Game/Blueprints/PickupActorInterface.Pickup`
  (params (AttachTo :type "SceneComponent Object Reference"))
  ;[1 1 1] Slightly altered BP_Pickup functionality, Input must be enabled and disabled to allow for the grip keys on the controllers to be pressed. Also gets and sets the Hand Name so that only THAT hands keys can be pressed.
  ;;[0 0 0] Drop and Pickup
  (`self.EnableInput` (`GameplayStatics.GetPlayerController` 0))
  (`PrimitiveComponent.SetSimulatePhysics` (`self.Body`) false)
  (`SceneComponent.K2_AttachToComponent` (`self.K2_GetRootComponent`) AttachTo "None" "SnapToTarget" "SnapToTarget" "KeepWorld" false)
  (bind _asbp_motion_controller (cast `/Game/Blueprints/BP_MotionController` (`ActorComponent.GetOwner` AttachTo)))
  (set `self.HandName` (`|GetEnumeratorNameAsString` (`/Game/Blueprints/BP_MotionController.Hand` _asbp_motion_controller))))

(event `/Game/Blueprints/PickupActorInterface.Drop`
  ;[1 1 1] Slightly altered BP_Pickup functionality, Input must be enabled and disabled to allow for the grip keys on the controllers to be pressed. Also gets and sets the Hand Name so that only THAT hands keys can be pressed.
  (`self.K2_DestroyActor`)
  ;;[0 0 0] Drop and Pickup
  (`self.DisableInput` (`GameplayStatics.GetPlayerController` 0))
  (`PrimitiveComponent.SetSimulatePhysics` (`self.Body`) true)
  (`self.K2_DetachFromActor` "KeepWorld" "KeepWorld" "KeepWorld"))

(event `InputAction|ActionSwap`
  (params (Key :type "Key Structure"))
  ;[1 1 1] Change Drill bit
  (:`Pressed`
    (if (`self.DrillBit?`)
      (`SceneComponent.SetHiddenInGame` (`self.DrillBit`) true false)
      (set `self.DrillBit?` false)
      (else
        (`SceneComponent.SetHiddenInGame` (`self.DrillBit`) false false)
        (set `self.DrillBit?` true)))))

(event `InputAction|ActionRightTrigger`
  (params (Key :type "Key Structure"))
  ;[1 1 1] Makes sure that only the GRIP buttons on the correct hand are being used to USE the Drill.
  (:`Pressed`
    (if (`KismetStringLibrary.EqualEqual_StrStr` (`self.HandName`) "Right")
      (if (`self.DrillBit?`) :!label _label
        ;[1 1 1] Drill Bit
        (for _array_element (`PrimitiveComponent.GetOverlappingActors` (`self.DrillBitCollision`) "/Game/Blueprints/BP_Holes.BP_Holes_C")
          (if (`Actor.bHidden` _array_element)
            (bind _asbp_holes (cast `/Game/Blueprints/BP_Holes` _array_element))
            (`/Game/Blueprints/BP_Holes.AddHole` _asbp_holes)))
        (else
          ;[1 1 1] For Each object being overlapped by the Drill collider, see if it has the "Bolt" Actor Tag, if true see if it is already hidden, if true, Hide, if not true, Unhide. Then, Get Panel with tag and cast to it, then remove (or add) the Bolts to the list. Panel checks to make sure ALL BOLTS are removed before IT can be removed.
          (`GameplayStatics.SpawnSoundAttached` "/Game/Import/Sounds/drill_01.drill_01" (`self.HexCollision`) "None" (0.0 0.0 0.0) (struct) "KeepRelativeOffset" false 1.0 1.0 0.0 null null)
          (for _array_element_2 (`PrimitiveComponent.GetOverlappingActors` (`self.HexCollision`) null)
            (if (`self.ActorHasTag` _array_element_2 "Bolt")
              (bind _output_get (set `self.BoltSelected` _array_element_2))
              (if (not (`Actor.bHidden` _array_element_2))
                (bind _asbp_bolt (cast `/Game/Blueprints/BP_Bolt` _output_get))
                (`/Game/Blueprints/BP_Bolt.RemoveBolt` _asbp_bolt)
                (else
                  (bind _asbp_bolt_2 (cast `/Game/Blueprints/BP_Bolt` _output_get))
                  (`/Game/Blueprints/BP_Bolt.AddBolt` _asbp_bolt_2))))))))))

(event `InputAction|ActionLeftTrigger`
  (params (Key :type "Key Structure"))
  ;[1 1 1] Makes sure that only the GRIP buttons on the correct hand are being used to USE the Drill.
  (:`Pressed`
    (if (`KismetStringLibrary.EqualEqual_StrStr` (`self.HandName`) "Left")
      (goto _label))))

(fn `UserConstructionScript`
  (bind _outactors (`GameplayStatics.GetAllActorsWithTag` "Panel"))
  (set `self.PanelList` _outactors))
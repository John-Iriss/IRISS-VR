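; BP_SwitchGear is a switchgear actor whose three conductive boxes can be switched between powered and unpowered states.
; On BeginPlay it spawns a BP_SwitchPanel at its own transform and attaches it to itself.
; PowerOn and PowerOff events set or clear the conductive component tag on the boxes, so power state is carried by tags.
; The construction script sets the actor's type tag.
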(event `self.ReceiveBeginPlay`
  (bind _returnvalue (`|SpawnActorFromClass` :`Class` "/Game/Blueprints/BP_SwitchPanel.BP_SwitchPanel_C" :`SpawnTransform` (`self.GetTransform` self) :`CollisionHandlingOverride` "Undefined" :`TransformScaleMethod` "OverrideRootScale" :`Instigator` null))
  (`self.K2_AttachToActor` _returnvalue self "None" "SnapToTarget" "KeepRelative" "KeepRelative" true))

(event `PowerOff`
  (`KismetArrayLibrary.Array_Clear` (`ActorComponent.ComponentTags` (`self.ConductiveBox`)))
  (`KismetArrayLibrary.Array_Clear` (`ActorComponent.ComponentTags` (`self.ConductiveBox_2`)))
  (`KismetArrayLibrary.Array_Clear` (`ActorComponent.ComponentTags` (`self.ConductiveBox_3`))))

(event `PowerOn`
  (bind _array (`|MakeArray` (`self.Conductive Tag`)))
  (set `ActorComponent.ComponentTags` _array (`self.ConductiveBox_3`))
  (set `ActorComponent.ComponentTags` _array (`self.ConductiveBox_2`))
  (set `ActorComponent.ComponentTags` _array (`self.ConductiveBox`)))

(fn `UserConstructionScript`
  (set `self.Tags` (`|MakeArray` (`self.TypeTag`))))
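; BP_SwitchGear_2 is a switchgear actor whose construction script tags its components for identification.
; The front internals and internals box meshes receive a conductive tag, and the scene root receives a type tag.
; BeginPlay is empty.
; Disconnected event-graph logic would spawn and attach a switch panel at the door socket and a switch at the handle socket, but never runs.
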(event `self.ReceiveBeginPlay`)

(fn `UserConstructionScript`
  (bind _array (`|MakeArray` (`self.Conductive Tag`)))
  (set `ActorComponent.ComponentTags` _array (`self.SwitchGear_Front_Internals`))
  (set `ActorComponent.ComponentTags` _array (`self.SwitchGear_Internals_Box`))
  (set `ActorComponent.ComponentTags` (`|MakeArray` (`self.TypeTag`)) (`self.DefaultSceneRoot`)))
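; BP_Bolt is a bolt actor that can be added to or removed from a parent switch panel.
; Its construction script sets its tag and caches the parent actor, so it expects to live as a child actor of a BP_SwitchPanel.
; AddBolt and RemoveBolt show or hide the bolt, then cast the parent to BP_SwitchPanel and pass the bolt to the panel's matching function.
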(event `AddBolt`
  (`self.SetActorHiddenInGame` false)
  (bind _asbp_switch_panel (cast `/Game/Blueprints/BP_SwitchPanel` (`self.Parent`)))
  (`/Game/Blueprints/BP_SwitchPanel.Add Bolt` _asbp_switch_panel self))

(event `RemoveBolt`
  (`self.SetActorHiddenInGame` true)
  (bind _asbp_switch_panel (cast `/Game/Blueprints/BP_SwitchPanel` (`self.Parent`)))
  (`/Game/Blueprints/BP_SwitchPanel.Remove Bolt` _asbp_switch_panel self))

(fn `UserConstructionScript`
  (set `self.Tags` (`|MakeArray` (`self.Tag`)))
  (set `self.Parent` (`self.GetParentActor`)))
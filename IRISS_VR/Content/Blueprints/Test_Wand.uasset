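; Test wand prop for motion controller pickup that lights up when touching components tagged "Conductive".
; Pickup disables mesh physics and attaches the root to the given component, while Drop restores physics and detaches.
; Box overlap events switch the PointLight on and off by checking only the entering or leaving component, so leaving one conductor darkens it even if others still overlap.
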(event `/Game/Blueprints/PickupActorInterface.Pickup`
  (params (AttachTo :type "SceneComponent Object Reference"))
  ;[1 1 1] Standard motion controller pickup and drop
  (`PrimitiveComponent.SetSimulatePhysics` (`self.StaticMeshComponent`) false)
  (`SceneComponent.K2_AttachToComponent` (`self.K2_GetRootComponent`) AttachTo "None" "KeepWorld" "KeepWorld" "KeepWorld" true))

(event `self.Box.OnComponentBeginOverlap`
  (params (OverlappedComponent :type "PrimitiveComponent Object Reference") (OtherActor :type "Actor Object Reference") (OtherComp :type "PrimitiveComponent Object Reference") (OtherBodyIndex :type Integer) (bFromSweep :type Boolean) (SweepResult :type "HitResult Structure (by ref)"))
  ;[1 1 1] If overlapping a conductive component Turn on Light, else turn off Light
  (for _ (`PrimitiveComponent.GetOverlappingComponents` (`self.Box`))
    (if (`ActorComponent.ComponentHasTag` OtherComp "Conductive")
      (`LightComponent.SetIntensity` (`self.PointLight`) 10.0))))

(event `/Game/Blueprints/PickupActorInterface.Drop`
  ;[1 1 1] Standard motion controller pickup and drop
  (`PrimitiveComponent.SetSimulatePhysics` (`self.StaticMeshComponent`) true)
  (`self.K2_DetachFromActor` "KeepWorld" "KeepWorld" "KeepWorld"))

(event `self.Box.OnComponentEndOverlap`
  (params (OverlappedComponent :type "PrimitiveComponent Object Reference") (OtherActor :type "Actor Object Reference") (OtherComp :type "PrimitiveComponent Object Reference") (OtherBodyIndex :type Integer))
  ;[1 1 1] If overlapping a conductive component Turn on Light, else turn off Light
  (if (`ActorComponent.ComponentHasTag` OtherComp "Conductive")
    (`LightComponent.SetIntensity` (`self.PointLight`) 0.0)))

(fn `UserConstructionScript`)
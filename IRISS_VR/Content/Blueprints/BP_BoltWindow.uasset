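; BP_BoltWindow is a bolt actor that can be shown or hidden and reports its state to an owning BP_CAP_ENV_12.
; AddBolt unhides the actor and RemoveBolt hides it, then each casts its Parent reference to BP_CAP_ENV_12 and passes itself to the matching function there.
; The construction script only calls its parent class version, and BeginPlay, overlap and Tick are unused.
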(event `self.AddBolt`
  (`self.SetActorHiddenInGame` false)
  (bind _asbp_cap_env_12 (cast `/Game/Blueprints/Windows/BP_CAP_ENV_12` (`self.Parent`)))
  (`/Game/Blueprints/Windows/BP_CAP_ENV_12.Add Bolt` _asbp_cap_env_12 self))

(event `self.RemoveBolt`
  (`self.SetActorHiddenInGame` true)
  (bind _asbp_cap_env_12 (cast `/Game/Blueprints/Windows/BP_CAP_ENV_12` (`self.Parent`)))
  (`/Game/Blueprints/Windows/BP_CAP_ENV_12.Remove Bolt` _asbp_cap_env_12 self))

(fn `UserConstructionScript`
  (`parent.UserConstructionScript`))
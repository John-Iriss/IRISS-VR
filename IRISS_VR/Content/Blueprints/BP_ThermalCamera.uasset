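; A hand-held thermal camera pickup that shows a thermal view and a °F readout.
; Pickup and Drop toggle physics, attachment and input, and the swap action cycles Iron, Rainbow and Blue scene captures with matching materials.
; At BeginPlay and while the right trigger is held, it samples the Iron render target's center pixel, lerping red and green into displayed temperature.
; It samples Iron in every palette, and the adjusted Temp variable never reaches the display.
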(event `self.ReceiveBeginPlay`
  ;[1 1 1] Deactivate Other Render targets and set initial temp
  (`ActorComponent.Deactivate` (`self.SceneCapture_Rainbow`))
  (`ActorComponent.Deactivate` (`self.SceneCaptureBlue`))
  ;[0.3408 0.9402 1] Grab color of pixel in middle of Render Target Texture, convert color to temp HOLY SHIT IT ACTUALLY WORKS
  (bind _returnvalue (`KismetRenderingLibrary.ReadRenderTargetRawPixel` "/Game/FX/ThermalVisionFX/Materials/RT_Thermal_Iron.RT_Thermal_Iron" 256 256 :!label _label))
  (bind (_r _g _b) (`KismetMathLibrary.BreakColor` _returnvalue))
  (bind _output_get (set `self.Temp` (* (+ _r _g _b) 100.0)))
  (if (<= _output_get 20.0)
    (set `self.Temp` (+ (`self.Temp`) 50.0))
    (elif (<= _output_get 30.0)
      (set `self.Temp` (+ (`self.Temp`) 40.0))
      (elif (<= _output_get 40.0)
        (set `self.Temp` (+ (`self.Temp`) 30.0))
        (elif (>= _output_get 150.0)
          (set `self.Temp` (- (`self.Temp`) 50.0))
          (elif (>= _output_get 120.0)
            (set `self.Temp` (- (`self.Temp`) 30.0)))))))
  (bind (_r_2 _g_2) (`KismetMathLibrary.BreakColor` _returnvalue))
  (`TextRenderComponent.K2_SetText` (`self.Text_Temp`) (`KismetTextLibrary.Conv_StringToText` (`KismetStringLibrary.Concat_StrStr` (`KismetTextLibrary.Conv_TextToString` (`KismetTextLibrary.Conv_DoubleToText` (`KismetMathLibrary.Lerp` 50.0 95.0 (/ (+ _r_2 _g_2) 2.0)) "HalfToEven" false true 1 324 1 1)) "°F"))))

(event `/Game/Blueprints/PickupActorInterface.Pickup`
  (params (AttachTo :type "SceneComponent Object Reference"))
  ;[1 1 1] Slightly altered BP_Pickup functionality, Input must be enabled and disabled to allow for the grip keys on the controllers to be pressed. Also gets and sets the Hand Name so that only THAT hands keys can be pressed.
  ;;[0 0 0] Drop and Pickup
  (`self.EnableInput` (`GameplayStatics.GetPlayerController` 0))
  (`PrimitiveComponent.SetSimulatePhysics` (`self.Body`) false)
  (`SceneComponent.K2_AttachToComponent` (`self.K2_GetRootComponent`) AttachTo "None" "SnapToTarget" "SnapToTarget" "KeepWorld" false))

(event `self.ReceiveTick`
  (params (DeltaSeconds :type "Float (single-precision)"))
  ;[0.3408 0.9402 1] Grab color of pixel in middle of Render Target Texture, convert color to temp HOLY SHIT IT ACTUALLY WORKS
  (`/Engine/EditorBlueprintResources/StandardMacros.Gate` true :!label _label_2
    (:`Exit`
      (goto _label))))

(event `/Game/Blueprints/PickupActorInterface.Drop`
  ;[1 1 1] Slightly altered BP_Pickup functionality, Input must be enabled and disabled to allow for the grip keys on the controllers to be pressed. Also gets and sets the Hand Name so that only THAT hands keys can be pressed.
  ;;[0 0 0] Drop and Pickup
  (`self.DisableInput` (`GameplayStatics.GetPlayerController` 0))
  (`PrimitiveComponent.SetSimulatePhysics` (`self.Body`) true)
  (`self.K2_DetachFromActor` "KeepWorld" "KeepWorld" "KeepWorld"))

(event `InputAction|ActionRightTrigger`
  (params (Key :type "Key Structure"))
  ;[0.3408 0.9402 1] Grab color of pixel in middle of Render Target Texture, convert color to temp HOLY SHIT IT ACTUALLY WORKS
  (:`Pressed`
    (goto _label_2 :!via `Open`))
  (:`Released`
    (goto _label_2 :!via `Close`)))

(event `InputAction|ActionSwap`
  (params (Key :type "Key Structure"))
  (bind _thermalview (`self.ThermalView`))
  ;[1 1 1] Thermal Gradient Switch
  (:`Pressed`
    (switch `int` (`self.ThermalMap`)
      (:`0`
        (`ActorComponent.Deactivate` (`self.SceneCapture_Iron`))
        (`ActorComponent.Activate` (`self.SceneCapture_Rainbow`) false)
        (`PrimitiveComponent.SetMaterial` _thermalview 0 "/Game/FX/ThermalVisionFX/Materials/MI_ThermalCamera_Rainbow.MI_ThermalCamera_Rainbow")
        (`PrimitiveComponent.SetMaterial` (`self.Temp_Gradiant`) 0 "/Game/Materials/M_ThermalGradient_Rainbow.M_ThermalGradient_Rainbow")
        (set `self.ThermalMap` 1))
      (:`1`
        (`ActorComponent.Deactivate` (`self.SceneCapture_Rainbow`))
        (`ActorComponent.Activate` (`self.SceneCaptureBlue`) false)
        (`PrimitiveComponent.SetMaterial` _thermalview 0 "/Game/FX/ThermalVisionFX/Materials/MI_ThermalCamera_Blue.MI_ThermalCamera_Blue")
        (`PrimitiveComponent.SetMaterial` (`self.Temp_Gradiant`) 0 "/Game/Materials/M_ThermalGradient_Blue.M_ThermalGradient_Blue")
        (set `self.ThermalMap` 2))
      (:`2`
        (`ActorComponent.Deactivate` (`self.SceneCaptureBlue`))
        (`ActorComponent.Activate` (`self.SceneCapture_Iron`) false)
        (`PrimitiveComponent.SetMaterial` _thermalview 0 "/Game/FX/ThermalVisionFX/Materials/MI_ThermalCamera_Iron.MI_ThermalCamera_Iron")
        (`PrimitiveComponent.SetMaterial` (`self.Temp_Gradiant`) 0 "/Game/Materials/M_ThermalGradient_Iron.M_ThermalGradient_Iron")
        (set `self.ThermalMap` 0)))))

(fn `UserConstructionScript`
  (set `self.ThermalMap` 0))
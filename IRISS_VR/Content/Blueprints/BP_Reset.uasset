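; BP_Reset is a pickup-triggered actor that brings up the gear selection menu.
; Its construction script searches for actors tagged "Menu" and stores the transform of the last one found as MenuLocation.
; Pickup turns the cube green and spawns BP_GearSelectionMenu at that transform.
; A delayed switch back to red is left unconnected, and GetLocationForMenu is an empty stub.
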(event `/Game/Blueprints/PickupActorInterface.Pickup`
  (params (AttachTo :type "SceneComponent Object Reference"))
  (`PrimitiveComponent.SetMaterial` (`self.Cube`) 0 "/Game/Materials/Green.Green")
  (`|SpawnActorFromClass` "/Game/Blueprints/BP_GearSelectionMenu.BP_GearSelectionMenu_C" (`self.MenuLocation`) "Undefined" "OverrideRootScale" null null))

(fn `GetLocationForMenu`
  (params (MenuLocation :type "Transform Structure")))

(fn `UserConstructionScript`
  (bind _outactors (`GameplayStatics.GetAllActorsWithTag` "Menu"))
  (for _array_element _outactors
    (set `self.MenuLocation` (`self.GetTransform` _array_element))))
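; ItemRecovery is a volume actor that returns items lost outside the scene.
; On BeginPlay it caches the world location of the first SpawnPoint actor, assuming only one exists, as the restore point.
; Any overlapping actor that is not another ItemRecovery is then moved to that point without sweeping.
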(event `self.ReceiveBeginPlay`
  ;[1 1 1] At Start, Get all Spawn Point Actors (only one) and get its start location. This is used to return items that have been lost outside of the scene.
  (bind _outactors (`GameplayStatics.GetAllActorsOfClass` "/Game/Blueprints/SpawnPoint.SpawnPoint_C"))
  (set `self.RestorePoint` (`SceneComponent.K2_GetComponentLocation` (`/Game/Blueprints/SpawnPoint.DefaultSceneRoot` (`|GetArrayItem` _outactors)))))

(event `self.ReceiveActorBeginOverlap`
  (params (OtherActor :type "Actor Object Reference"))
  ;[1 1 1] If an object overlaps one of these areas (ItemRecovery), set that actors location to the Recovery Point.
  (if (!= (`GameplayStatics.GetObjectClass` OtherActor) "ItemRecovery_C")
    (`self.K2_SetActorLocation` OtherActor (`self.RestorePoint`) false true)))

(fn `UserConstructionScript`)
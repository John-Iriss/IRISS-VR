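; BP_LockoutTag is a VR-grabbable lockout tag that locks switches and reports tagging progress to BP_GameMode_IRISS.
; Pickup attaches it to the motion controller's child socket, and Drop restores physics.
; Overlapping a "LockOut"-tagged root snaps it on, plays a rotation timeline and locks every "Switch"-tagged actor.
; Picking up a locked tag reverses the rotation and unlocks them, reporting removal once and only after SafeToRemove.
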(event `/Game/Blueprints/PickupActorInterface.Pickup`
  (params (AttachTo :type "SceneComponent Object Reference"))
  (bind _returnvalue (`SceneComponent.GetChildComponent` (cast `MotionControllerComponent` AttachTo :!pure true) 0))
  ;[0 0 0] Drop and Pickup
  (if (not (`self.IsLocked`))
    (`PrimitiveComponent.SetSimulatePhysics` (`self.LockoutBase`) false)
    (`SceneComponent.K2_AttachToComponent` (`self.K2_GetRootComponent`) _returnvalue "LockTag" "SnapToTarget" "SnapToTarget" "KeepWorld" false)
    (else
      (`self.RemoveTag`)
      (`self.K2_DetachFromActor` "KeepWorld" "KeepWorld")
      (`PrimitiveComponent.SetSimulatePhysics` (`self.LockoutBase`) false)
      (`SceneComponent.K2_AttachToComponent` (`self.K2_GetRootComponent`) _returnvalue "LockTag" "SnapToTarget" "SnapToTarget" "KeepWorld" false))))

(event `self.ReceiveBeginPlay`
  (`self.EnableInput` (`GameplayStatics.GetPlayerController` 0)))

(event `/Game/Blueprints/PickupActorInterface.Drop`
  ;[0 0 0] Drop and Pickup
  (`PrimitiveComponent.SetSimulatePhysics` (`self.LockoutBase`) true)
  (`self.K2_DetachFromActor` "KeepWorld" "KeepWorld" "KeepWorld"))

(event `self.CollisionBox.OnComponentBeginOverlap`
  (params (OverlappedComponent :type "PrimitiveComponent Object Reference") (OtherActor :type "Actor Object Reference") (OtherComp :type "PrimitiveComponent Object Reference") (OtherBodyIndex :type Integer) (bFromSweep :type Boolean) (SweepResult :type "HitResult Structure (by ref)"))
  ;[1 1 1] Attach Lockout Tag to Switch
  (if (not (`self.IsLocked`))
    (if (`ActorComponent.ComponentHasTag` (`Actor.RootComponent` OtherActor) "LockOut")
      (`self.K2_AttachToActor` OtherActor "LockoutTag" "SnapToTarget" "SnapToTarget" "KeepRelative" false)
      (`self.AttachTag`)
      (`/Engine/EditorBlueprintResources/StandardMacros.DoOnce` false
        (:`Completed`
          (`/Game/Blueprints/BP_GameMode_IRISS.Tag On` (cast `/Game/Blueprints/BP_GameMode_IRISS` (`GameplayStatics.GetGameMode`) :!pure true)))))))

(event `AttachTag`
  ;[1 1 1] Play animation once attached
  (bind (_direction _rotationspeed) (`Timeline|Timeline_0` :!via `PlayFromStart`)
    (:`Update`
      (`SceneComponent.K2_SetRelativeRotation` (`self.RotationJoint`) (`KismetMathLibrary.RLerp` (`SceneComponent.RelativeRotation` (`self.RotationJoint`)) (struct) _rotationspeed) false false)
      (set `self.IsLocked` true)
      (bind _outactors (`GameplayStatics.GetAllActorsWithTag` "Switch"))
      (for _array_element _outactors
        (set `/Game/Blueprints/BP_Switch.Locked` true (cast `/Game/Blueprints/BP_Switch` _array_element :!pure true))))))

(event `SafeToRemove`
  (set `self.Safe?` true))

(event `RemoveTag`
  ;[1 1 1] Play animation once removed
  (bind (_direction _rotationspeed) (`Timeline|Timeline_1` :!via `PlayFromStart`)
    (:`Update`
      (`SceneComponent.K2_SetRelativeRotation` (`self.RotationJoint`) (`KismetMathLibrary.RLerp` (`SceneComponent.RelativeRotation` (`self.RotationJoint`)) (`self.StartingRotation`) _rotationspeed) false false))
    (:`Finished`
      (set `self.IsLocked` false)
      (bind _outactors (`GameplayStatics.GetAllActorsWithTag` "Switch"))
      (for _array_element _outactors
        (set `/Game/Blueprints/BP_Switch.Locked` false (cast `/Game/Blueprints/BP_Switch` _array_element :!pure true))
        (`/Engine/EditorBlueprintResources/StandardMacros.DoOnce` false :!label _label
          (:`Completed`
            (if (`self.Safe?`)
              (bind _asbp_game_mode_iriss (cast `/Game/Blueprints/BP_GameMode_IRISS` (`GameplayStatics.GetGameMode`)))
              (`/Game/Blueprints/BP_GameMode_IRISS.TagRemoved` _asbp_game_mode_iriss)
              (else
                (goto _label :!via `Reset`)))))))))

(fn `NewFunction_0`
  (params (Object :type "Object Object Reference"))
  (cast `MotionControllerComponent` Object))

(fn `UserConstructionScript`
  (set `self.StartingRotation` (`SceneComponent.RelativeRotation` (`self.RotationJoint`))))
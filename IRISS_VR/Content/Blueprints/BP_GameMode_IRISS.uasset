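; Game mode for a VR training sequence that walks the player through installing a window in a gear panel, from lockout to power-on.
; Each step event fires once through a DoOnce and updates the motion controller pawn's HUD with the next instruction.
; Step order is not enforced, except that the completion message requires the lockout tag to be removed first.
; Spawn events forward the chosen gear, window and template classes to their spawn-point actors found by class.
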(event `GearSelected`
  (`/Engine/EditorBlueprintResources/StandardMacros.DoOnce` false
    (:`Completed`
      (`/Game/Blueprints/MotionControllerPawn.ChangeHudText` (`self.PlayerRef`) "Please Select A Window"))))

(event `Window Selected`
  (`/Engine/EditorBlueprintResources/StandardMacros.DoOnce` false
    (:`Completed`
      (`/Game/Blueprints/MotionControllerPawn.ChangeHudText` (`self.PlayerRef`) "Approach the installation area"))))

(event `Entered Installation Area`
  (`/Engine/EditorBlueprintResources/StandardMacros.DoOnce` false
    (:`Completed`
      (`/Game/Blueprints/MotionControllerPawn.ChangeHudText` (`self.PlayerRef`) "Turn Off Power"))))

(event `self.ReceiveBeginPlay`
  (bind _asmotion_controller_pawn (cast `/Game/Blueprints/MotionControllerPawn` (`GameplayStatics.GetPlayerPawn` 0)))
  (set `self.PlayerRef` _asmotion_controller_pawn))

(event `PowerOff`
  (`/Engine/EditorBlueprintResources/StandardMacros.DoOnce` false
    (:`Completed`
      (`/Game/Blueprints/MotionControllerPawn.ChangeHudText` (`self.PlayerRef`) "Apply The Lockout Tag"))))

(event `Tag On`
  (`/Engine/EditorBlueprintResources/StandardMacros.DoOnce` false
    (:`Completed`
      (`/Game/Blueprints/MotionControllerPawn.ChangeHudText` (`self.PlayerRef`) "Remove Bolts From Panel"))))

(event `Bolts Removed`
  (`/Engine/EditorBlueprintResources/StandardMacros.DoOnce` false
    (:`Completed`
      (`/Game/Blueprints/MotionControllerPawn.ChangeHudText` (`self.PlayerRef`) "Remove Panel And Place On Table"))))

(event `SpawnGear`
  (params (GearToSpawn :type "Actor Class Reference"))
  (bind _outactors (`GameplayStatics.GetAllActorsOfClass` "/Game/Blueprints/BP_GearSpawn.BP_GearSpawn_C"))
  (`/Game/Blueprints/BP_GearSpawn.SpawnGear` _outactors GearToSpawn))

(event `Placed`
  (`/Engine/EditorBlueprintResources/StandardMacros.DoOnce` false
    (:`Completed`
      (`/Game/Blueprints/MotionControllerPawn.ChangeHudText` (`self.PlayerRef`) "Apply Template Sticker"))))

(event `SpawnWindow`
  (params (Window :type "Actor Class Reference") (Template :type "Actor Class Reference"))
  (`|ExecutionSequence`
    (:`then_0`
      (bind _outactors (`GameplayStatics.GetAllActorsOfClass` "/Game/Blueprints/BP_WindowSpawn.BP_WindowSpawn_C"))
      (`/Game/Blueprints/BP_WindowSpawn.SpawnWindow` _outactors Window))
    (:`then_1`
      (bind _outactors_2 (`GameplayStatics.GetAllActorsOfClass` "/Game/Blueprints/BP_TemplateSpawn.BP_TemplateSpawn_C"))
      (`/Game/Blueprints/BP_TemplateSpawn.SpawnTemplate` _outactors_2 Template))))

(event `TemplateOn`
  (`/Engine/EditorBlueprintResources/StandardMacros.DoOnce` false
    (:`Completed`
      (`/Game/Blueprints/MotionControllerPawn.ChangeHudText` (`self.PlayerRef`) "Drill Out Holes And Cut Out Window "))))

(event `HoleCut`
  (`/Engine/EditorBlueprintResources/StandardMacros.DoOnce` false
    (:`Completed`
      (`/Game/Blueprints/MotionControllerPawn.ChangeHudText` (`self.PlayerRef`) "Remove Template Sticker"))))

(event `StickerRemoved`
  (`/Engine/EditorBlueprintResources/StandardMacros.DoOnce` false
    (:`Completed`
      (`/Game/Blueprints/MotionControllerPawn.ChangeHudText` (`self.PlayerRef`) "Apply Window To Panel"))))

(event `WindowOn`
  (`/Engine/EditorBlueprintResources/StandardMacros.DoOnce` false
    (:`Completed`
      (`/Game/Blueprints/MotionControllerPawn.ChangeHudText` (`self.PlayerRef`) "Bolt On Window"))))

(event `WindowBolted`
  (`/Engine/EditorBlueprintResources/StandardMacros.DoOnce` false
    (:`Completed`
      (`/Game/Blueprints/MotionControllerPawn.ChangeHudText` (`self.PlayerRef`) "Apply Panel To Gear"))))

(event `PanelOn`
  (`/Engine/EditorBlueprintResources/StandardMacros.DoOnce` false
    (:`Completed`
      (`/Game/Blueprints/MotionControllerPawn.ChangeHudText` (`self.PlayerRef`) "Bolt On Panel"))))

(event `PanelBolted`
  (`/Engine/EditorBlueprintResources/StandardMacros.DoOnce` false
    (:`Completed`
      (`/Game/Blueprints/MotionControllerPawn.ChangeHudText` (`self.PlayerRef`) "Remove Lockout Tag"))))

(event `TagRemoved`
  (`/Engine/EditorBlueprintResources/StandardMacros.DoOnce` false
    (:`Completed`
      (`/Game/Blueprints/MotionControllerPawn.ChangeHudText` (`self.PlayerRef`) "Turn On Power")
      (set `self.TagOff` true))))

(event `PowerOn`
  (if (`self.TagOff`)
    (`/Engine/EditorBlueprintResources/StandardMacros.DoOnce` false
      (:`Completed`
        (`/Game/Blueprints/MotionControllerPawn.ChangeHudText` (`self.PlayerRef`) "COMPLETED")))))

(fn `UserConstructionScript`
  (bind _outactors (`GameplayStatics.GetAllActorsOfClass` "/Game/Blueprints/BP_GearSpawn.BP_GearSpawn_C"))
  (set `self.SpawnPoint` (`|GetArrayItem` _outactors)))
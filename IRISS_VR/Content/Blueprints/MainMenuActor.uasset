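; VR main menu actor where motion controller overlaps pick an installation type, category and product before loading the Sample-2 level.
; Each button requires the earlier selections, uses a FlipFlop to swap its material and set its state, and the first two toggle child option texts.
; Once all three selections are set, the next actor overlap opens the level.
; Tick applies a temporary fix toggling CapText when CAPENV12Text shows without it.
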(event `self.ReceiveBeginPlay`)

(event `self.ReceiveTick`
  (params (DeltaSeconds :type "Float (single-precision)"))
  (bind _captext (`self.CapText`))
  (if (and (not (`SceneComponent.IsVisible` _captext)) (`SceneComponent.IsVisible` (`self.CAP-ENV-12Text`)))
    ;[1 1 1] Temp visibility solution for children
    (`SceneComponent.ToggleVisibility` _captext true)))

(event `self.ReceiveActorBeginOverlap`
  (params (OtherActor :type "Actor Object Reference"))
  (bind _capbutton (`self.CapButton`))
  (bind _installationbutton (`self.InstallationButton`))
  (bind _cap_env_12button (`self.CAP-ENV-12Button`))
  (if (and (`self.TypeSelected?`) (`self.CatigorySelected?`) (`self.ProductSelected?`))
    (`GameplayStatics.OpenLevel` "Sample-2")
    (elif (== (`GameplayStatics.GetObjectClass` OtherActor) "/Game/Blueprints/BP_MotionController.BP_MotionController_C")
      (if (`PrimitiveComponent.IsOverlappingActor` (`self.InstallationButton`) OtherActor)
        (set `self.InstallationTypeArray` (`|MakeArray` (`self.vpText`) (`self.CapText`) (`self.CustomText`)))
        (bind _isa (`/Engine/EditorBlueprintResources/StandardMacros.FlipFlop`)
          (:`A`
            (`PrimitiveComponent.SetMaterial` _installationbutton 0 "/Game/Materials/MenuButtonDark.MenuButtonDark"))
          (:`B`
            (`PrimitiveComponent.SetMaterial` _installationbutton 0 "/Game/Materials/MenuButton.MenuButton")))
        (set `self.TypeSelected?` _isa)
        (for _array_element (`self.InstallationTypeArray`)
          (`SceneComponent.ToggleVisibility` _array_element true)
          (`ActorComponent.ToggleActive` _array_element))
        (elif (and (`PrimitiveComponent.IsOverlappingActor` (`self.CapButton`) OtherActor) (`self.TypeSelected?`))
          (set `self.InstallationCatArray` (`|MakeArray` (`self.CAP-ENV-12Text`)))
          (bind _isa_2 (`/Engine/EditorBlueprintResources/StandardMacros.FlipFlop`)
            (:`A`
              (`PrimitiveComponent.SetMaterial` _capbutton 0 "/Game/Materials/MenuButtonDark.MenuButtonDark"))
            (:`B`
              (`PrimitiveComponent.SetMaterial` _capbutton 0 "/Game/Materials/MenuButton.MenuButton")))
          (set `self.CatigorySelected?` _isa_2)
          (for _array_element_2 (`self.InstallationCatArray`)
            (`SceneComponent.ToggleVisibility` _array_element_2 true)
            (`ActorComponent.ToggleActive` _array_element_2))
          (elif (and (`PrimitiveComponent.IsOverlappingActor` (`self.CAP-ENV-12Button`) OtherActor) (`self.TypeSelected?`) (`self.CatigorySelected?`))
            (bind _isa_3 (`/Engine/EditorBlueprintResources/StandardMacros.FlipFlop`)
              (:`A`
                (`PrimitiveComponent.SetMaterial` _cap_env_12button 0 "/Game/Materials/MenuButtonDark.MenuButtonDark"))
              (:`B`
                (`PrimitiveComponent.SetMaterial` _cap_env_12button 0 "/Game/Materials/MenuButton.MenuButton")))
            (set `self.ProductSelected?` _isa_3)))))))

(fn `UserConstructionScript`)
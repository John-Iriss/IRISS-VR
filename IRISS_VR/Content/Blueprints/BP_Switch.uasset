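; BP_Switch is an interactive power switch that toggles its parent BP_SwitchGear on or off when Pickup fires and it is not locked.
; Two chained timelines swing the handle joint out and back, then flip the Power state and red/green icon.
; It then notifies the switchgear, cached from the parent actor at construction, and BP_GameMode_IRISS.
; A DoOnce with no reset limits the game mode's power-off call to one time.
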(event `/Game/Blueprints/PickupActorInterface.Pickup`
  (params (AttachTo :type "SceneComponent Object Reference"))
  ;[1 1 1] Animate Switch and turn On/Off power
  (if (not (`self.Locked`))
    (if (`self.Power`)
      (bind (_direction _rotatespeed) (`Timeline|TurnOFF` :!via `PlayFromStart`)
        (:`Update`
          (`SceneComponent.K2_SetRelativeRotation` (`self.HandleJoint`) (`KismetMathLibrary.RLerp` (`SceneComponent.RelativeRotation` (`self.HandleJoint`)) (struct :`Pitch` 50.0) _rotatespeed) false false))
        (:`Finished`
          (bind (_direction_2 _rotatespeed_2) (`Timeline|TurnOFF2` :!via `PlayFromStart`)
            (:`Update`
              (`SceneComponent.K2_SetRelativeRotation` (`self.HandleJoint`) (`KismetMathLibrary.RLerp` (`SceneComponent.RelativeRotation` (`self.HandleJoint`)) (struct) _rotatespeed_2) false false))
            (:`Finished`
              (`PrimitiveComponent.SetMaterial` (`self.PowerIcon`) 0 "/Game/Materials/Red.Red")
              (set `self.Power` false)
              (bind _asbp_switch_gear (cast `/Game/Blueprints/SwitchGear/BP_SwitchGear` (`self.Parent`)))
              (`/Game/Blueprints/SwitchGear/BP_SwitchGear.PowerOff` _asbp_switch_gear)
              (`/Engine/EditorBlueprintResources/StandardMacros.DoOnce` false
                (:`Completed`
                  (`/Game/Blueprints/BP_GameMode_IRISS.PowerOff` (cast `/Game/Blueprints/BP_GameMode_IRISS` (`GameplayStatics.GetGameMode`) :!pure true))))))))
      (else
        (bind (_direction_3 _rotatespeed_3) (`Timeline|Timeline_0` :!via `PlayFromStart`)
          (:`Update`
            (`SceneComponent.K2_SetRelativeRotation` (`self.HandleJoint`) (`KismetMathLibrary.RLerp` (`SceneComponent.RelativeRotation` (`self.HandleJoint`)) (struct :`Pitch` 90.0) _rotatespeed_3) false false))
          (:`Finished`
            (bind (_direction_4 _rotatespeed_4) (`Timeline|Timeline_1` :!via `PlayFromStart`)
              (:`Update`
                (`SceneComponent.K2_SetRelativeRotation` (`self.HandleJoint`) (`KismetMathLibrary.RLerp` (`SceneComponent.RelativeRotation` (`self.HandleJoint`)) (struct) _rotatespeed_4) false false))
              (:`Finished`
                (`PrimitiveComponent.SetMaterial` (`self.PowerIcon`) 0 "/Game/Materials/Green.Green")
                (set `self.Power` true)
                (bind _asbp_switch_gear_old (cast `/Game/Blueprints/SwitchGear/BP_SwitchGear` (`self.Parent`)))
                (`/Game/Blueprints/SwitchGear/BP_SwitchGear.PowerOn` _asbp_switch_gear_old)
                (`/Game/Blueprints/BP_GameMode_IRISS.PowerOn` (cast `/Game/Blueprints/BP_GameMode_IRISS` (`GameplayStatics.GetGameMode`) :!pure true))))))))))

(fn `UserConstructionScript`
  (set `self.StartingRotation` (`SceneComponent.RelativeRotation` (`self.HandleJoint`)))
  (set `self.Parent` (`self.GetParentActor`)))
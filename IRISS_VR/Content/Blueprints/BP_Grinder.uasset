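; BP_Grinder is a hand-held grinder that a motion controller picks up to cut pieces out of a template.
; Pickup attaches it, enables input and records the hand, so that hand's trigger sets IsOn and the other's clears it.
; While on, overlapping a hidden Cutout-tagged actor calls Cutout on the first Template-tagged actor.
; Drop restores physics and disables input; sound playback and particle activation are unwired.
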(event OnComponentBeginOverlap(Box)
  (params (OverlappedComponent :type Primitive%20Component%20Object%20Reference) (OtherActor :type Actor%20Object%20Reference) (OtherComp :type Primitive%20Component%20Object%20Reference) (OtherBodyIndex :type Integer) (bFromSweep :type Boolean) (SweepResult :type Hit%20Result%20Structure%20%28by%20ref%29))
  ;[1 1 1] If the Grinder Hits or Overlaps a viable object when it is on, the grinder will spawn an audio clib at that location. If it is used on a template with "cut out"
  (if (Variables|Default|GetIsOn?)
    (for _array_element (Utilities|Array|MakeArray OtherActor)
      (if (Actor|ActorHasTag _array_element "Cutout")
        (bind _output_get (Variables|Default|SetCutoutPiece OtherActor))
        (if (Variables|/Script/Engine.Actor|GetbHidden _output_get)
          (bind _outactors (Actor|GetAllActorswithTag "Template"))
          (bind _asbp_template (Utilities|Casting|CastToBP_Template (Utilities|Array|Get(acopy) _outactors)))
          (Default|Cutout _asbp_template _output_get))))))

(event Custom|StopRun
  ;[1 1 1] If the Grinder Hits or Overlaps a viable object when it is on, the grinder will spawn an audio clib at that location. If it is used on a template with "cut out"
  ;;[1 1 1] There are several StopRun scripts in this BP that shut off the Particle System and Audio.
  (Components|Activation|Deactivate (Variables|Default|GetParticleSystem))
  (if (Utilities|IsValid (stale _returnvalue))
    _))

(event EventPickup
  (params (AttachTo :type Scene%20Component%20Object%20Reference))
  (bind _returnvalue (Components|GetOwner AttachTo))
  ;[1 1 1] Similar to Drill, allows object to be picked up, enables and disables input (so that the grinder activates) and sets the Hand Name Variable so only that hands buttons will trigger activation.
  (Input|EnableInput (Game|GetPlayerController 0))
  (Physics|SetSimulatePhysics (Variables|Default|GetBody) false)
  (Transformation|AttachComponentToComponent (VehicleSound|GetRootComponent) AttachTo "None" "SnapToTarget" "SnapToTarget" "KeepWorld" false)
  (Variables|Default|SetHandController _returnvalue)
  (bind _asbp_motion_controller (Utilities|Casting|CastToBP_MotionController _returnvalue))
  (Variables|Default|SetHandName (Utilities|String|EnumtoString (Variables|/Game/Blueprints/BP_MotionController.BP_MotionController_C|GetHand _asbp_motion_controller))))

(event EventDrop
  ;[1 1 1] Similar to Drill, allows object to be picked up, enables and disables input (so that the grinder activates) and sets the Hand Name Variable so only that hands buttons will trigger activation.
  (CallFunction|StopRun)
  (Input|DisableInput (Game|GetPlayerController 0))
  (Physics|SetSimulatePhysics (Variables|Default|GetBody) true)
  (Transformation|DetachFromActor "KeepWorld" "KeepWorld" "KeepWorld"))

(event Collision|EventActorEndOverlap
  (params (OtherActor :type Actor%20Object%20Reference)))

(event Input|ActionEvents|InputActionActionRightTrigger
  (params (Key :type Key%20Structure))
  ;[1 1 1] Make sure that input is only comming from the correct hand, sets the variable isOn?
  (:Pressed
    (if (Utilities|Enum|Equal(Enum) (Variables|Default|GetHandName) "Right")
      (Variables|Default|SetIsOn? true)
      (else
        (Variables|Default|SetIsOn? false)))))

(event Input|ActionEvents|InputActionActionLeftTrigger
  (params (Key :type Key%20Structure))
  ;[1 1 1] Make sure that input is only comming from the correct hand, sets the variable isOn?
  (:Pressed
    (if (Utilities|Enum|Equal(Enum) (Variables|Default|GetHandName) "Left")
      (Variables|Default|SetIsOn? true)
      (else
        (Variables|Default|SetIsOn? false)))))

(fn ConstructionScript)
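; BP_Trigger1 is a trigger actor that reports interactions with actors tagged "Panel" to BP_GameMode_IRISS, apparently for panel placement.
; Its Box component's begin overlap, end overlap and hit events each check the tag, then cast the game mode and call Placed.
; All three events make the same argument-free call, so the game mode is not told whether a panel entered, left or hit the box.
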(event `self.Box.OnComponentBeginOverlap`
  (params (OverlappedComponent :type "PrimitiveComponent Object Reference") (OtherActor :type "Actor Object Reference") (OtherComp :type "PrimitiveComponent Object Reference") (OtherBodyIndex :type Integer) (bFromSweep :type Boolean) (SweepResult :type "HitResult Structure (by ref)"))
  (if (`self.ActorHasTag` OtherActor "Panel")
    (`/Game/Blueprints/BP_GameMode_IRISS.Placed` (cast `/Game/Blueprints/BP_GameMode_IRISS` (`GameplayStatics.GetGameMode`) :!pure true))))

(event `self.Box.OnComponentEndOverlap`
  (params (OverlappedComponent :type "PrimitiveComponent Object Reference") (OtherActor :type "Actor Object Reference") (OtherComp :type "PrimitiveComponent Object Reference") (OtherBodyIndex :type Integer))
  (if (`self.ActorHasTag` OtherActor "Panel")
    (`/Game/Blueprints/BP_GameMode_IRISS.Placed` (cast `/Game/Blueprints/BP_GameMode_IRISS` (`GameplayStatics.GetGameMode`) :!pure true))))

(event `self.Box.OnComponentHit`
  (params (HitComponent :type "PrimitiveComponent Object Reference") (OtherActor :type "Actor Object Reference") (OtherComp :type "PrimitiveComponent Object Reference") (NormalImpulse :type "Vector Structure") (Hit :type "HitResult Structure (by ref)"))
  (if (`self.ActorHasTag` OtherActor "Panel")
    (`/Game/Blueprints/BP_GameMode_IRISS.Placed` (cast `/Game/Blueprints/BP_GameMode_IRISS` (`GameplayStatics.GetGameMode`) :!pure true))))

(fn `UserConstructionScript`)